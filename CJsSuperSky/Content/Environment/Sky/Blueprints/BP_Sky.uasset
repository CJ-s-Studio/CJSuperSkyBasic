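; Sky actor that runs a looping day-night cycle with sun, moon and rotating stars.
; Each tick advances GlobalTimeOfDay by a fixed, frame-rate-dependent step, then rotates both lights using sunrise and sunset times derived from DaylightDuration.
; Light heights, taken from direction dot products, drive curve-based colours on lights and dynamic materials, plus sun brightness.
; Construction also refreshes the sky; eclipse and light-priority functions are unfinished stubs.
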(event `self.ReceiveTick`
  (params (DeltaSeconds :type "Float (single-precision)"))
  ; Read me
  (`self.DayNightCycle`)
  (`self.UpdateSky`))

(fn `CalculateEclipses`
  ; Eclipse Logic
)

(fn `DayNightCycle`
  (if (< (/ (`self.GlobalTimeOfDay`) 24.0) 1.0)
    (set `self.GlobalTimeOfDay` (+ (`self.GlobalTimeOfDay`) (* (/ 0.01 (* (`self.DayDuration`) 60.0)) 24.0)))
    (else
      (set `self.GlobalTimeOfDay` 0.0))))

(fn `GetSunRiseTime`
  (returns (Time :type "Float (double-precision)"))
  (return (`KismetMathLibrary.MapRangeUnclamped` (`self.DaylightDuration`) 0.25 0.75 9.0 3.0)))

(fn `GetSunSetTime`
  (returns (Time :type "Float (double-precision)"))
  (return (`KismetMathLibrary.MapRangeUnclamped` (`self.DaylightDuration`) 0.25 0.75 15.0 21.0)))

(fn `Update Stars`
  (`SceneComponent.K2_SetRelativeRotation` (`self.SkyGlobalPositionOffset`) (`KismetMathLibrary.MakeRotator` (+ (* 0.0 -1.0) 90.0) (* 0.0 -1.0) (+ 0.0 180.0)) false false)
  (`SceneComponent.K2_SetRelativeRotation` (`self.SkyStars`) (`KismetMathLibrary.MakeRotator` 0.0 0.0 (`KismetMathLibrary.MapRangeClamped` (`self.GlobalTimeOfDay`) 0.0 24.0 0.0 360.0)) false false))

(fn `UpdateDirectionalLightPriority`
  ; Updates Directional Light Priority
  (if (> (`LightComponentBase.Intensity` (`self.SunLight`)) (`LightComponentBase.Intensity` (`self.MoonLight`)))
    _))

(fn `UpdateMoonHeight`
  (set `self.MoonHeight` (`KismetMathLibrary.Dot_VectorVector` (0.0 0.0 -1.0) (`KismetMathLibrary.Conv_RotatorToVector` (`SceneComponent.K2_GetComponentRotation` (`self.MoonLight`))))))

(fn `UpdateMoonMaterial`
  (bind _returnvalue (* (`KismetMathLibrary.MapRangeClamped` (`self.MoonHeight`) 0.0 0.5 0.0 1.0) (- 1.0 0.0)))
  ; Updates Moon Material
  (`MaterialInstanceDynamic.SetVectorParameterValue` (`self.MoonMaterial`) "SunDirection" (`KismetMathLibrary.Conv_VectorToLinearColor` (* (`SceneComponent.GetForwardVector` (`self.SunLight`)) -1.0)))
  (`MaterialInstanceDynamic.SetVectorParameterValue` (`self.MoonMaterial`) "MoonColor" (`CurveLinearColor.GetLinearColorValue` (`self.MoonColorCurve`) _returnvalue))
  (`LightComponent.SetLightColor` (`self.MoonLight`) (`CurveLinearColor.GetLinearColorValue` (`self.MoonLightColorCurve`) _returnvalue) true))

(fn `UpdateMoonSettings`
  (bind _returnvalue (* (`self.MoonScale`) 6000.0))
  ; Moon Rotation/Scale Updating
  (`SceneComponent.K2_SetRelativeRotation` (`self.MoonLight`) (`KismetMathLibrary.MakeRotator` 0.0 0.0 (`KismetMathLibrary.SelectFloat` (`KismetMathLibrary.Lerp` 180.0 360.0 (`KismetMathLibrary.MapRangeClamped` (`self.GlobalTimeOfDay`) (`self.GetSunRiseTime`) (`self.GetSunSetTime`) 0.0 1.0)) (`KismetMathLibrary.Lerp` 0.0 180.0 (`KismetMathLibrary.SelectFloat` (`KismetMathLibrary.MapRangeClamped` (`self.GlobalTimeOfDay`) (`self.GetSunSetTime`) (+ (`self.GetSunRiseTime`) 24.0) 0.0 1.0) (`KismetMathLibrary.MapRangeClamped` (`self.GlobalTimeOfDay`) (- (`self.GetSunSetTime`) 24.0) (`self.GetSunRiseTime`) 0.0 1.0) (> (`self.GlobalTimeOfDay`) (`self.GetSunSetTime`)))) (not (or (> (`self.GlobalTimeOfDay`) (`self.GetSunSetTime`)) (< (`self.GlobalTimeOfDay`) (`self.GetSunRiseTime`)))))) false false)
  (`SceneComponent.SetRelativeScale3D` (`self.Moon`) (`KismetMathLibrary.MakeVector` _returnvalue _returnvalue _returnvalue))
  (`self.UpdateMoonHeight`))

(fn `UpdateSky`
  (`|ExecutionSequence`
    (:`then_0`
      (`self.UpdateSunSettings`))
    (:`then_1`
      (`self.UpdateSunMaterial`))
    (:`then_2`
      (`self.UpdateMoonSettings`))
    (:`then_3`
      (`self.UpdateMoonMaterial`))
    (:`then_4`
      (`self.Update Stars`))))

(fn `UpdateSunHeight`
  (set `self.SunHeight` (`KismetMathLibrary.Dot_VectorVector` (0.0 0.0 -1.0) (`KismetMathLibrary.Conv_RotatorToVector` (`SceneComponent.K2_GetComponentRotation` (`self.SunLight`))))))

(fn `UpdateSunMaterial`
  (bind _returnvalue (- 1.0 0.0))
  (bind _sunmaterial (`self.SunMaterial`))
  (bind _returnvalue_2 (`CurveLinearColor.GetLinearColorValue` (`self.EclipseColorCurve`) 0.0))
  (bind _returnvalue_3 (`KismetMathLibrary.MapRangeClamped` (`self.SunHeight`) 0.0 0.5 0.0 1.0))
  ; Updates Sun Material
  (`MaterialInstanceDynamic.SetVectorParameterValue` _sunmaterial "SunColor" (* (`CurveLinearColor.GetLinearColorValue` (`self.SunColorCurve`) (* _returnvalue _returnvalue_3)) _returnvalue_2))
  (`MaterialInstanceDynamic.SetScalarParameterValue` _sunmaterial "Brightness" (* (`KismetMathLibrary.MapRangeClamped` _returnvalue_3 0.0 0.5 5.0 10.0) (`KismetMathLibrary.MapRangeClamped` _returnvalue 0.0 1.0 0.9 1.0)))
  (`LightComponent.SetLightColor` (`self.SunLight`) (* (`CurveLinearColor.GetLinearColorValue` (`self.SunLightColorCurve`) _returnvalue_3) _returnvalue_2) true))

(fn `UpdateSunSettings`
  (bind _returnvalue (* (`self.SunScale`) 920000.0))
  ; Sets the Rotation/Scale and Brightess of Sun
  (`self.UpdateSunHeight`)
  (`LightComponent.SetIntensity` (`self.SunLight`) (* (`KismetMathLibrary.FClamp` (`self.SunHeight`) 0.1) (`KismetMathLibrary.MapRangeClamped` (`KismetMathLibrary.FClamp` (- 1.0 0.0) 0.5) 0.5 1.0 2.5 50.0)))
  (set `self.LocalTimeOfDay` (`KismetMathLibrary.FWrap` (+ (`self.GlobalTimeOfDay`) (* (/ 0.0 360.0) 24.0)) 0.0 24.0))
  (`SceneComponent.K2_SetRelativeRotation` (`self.SunLight`) (`KismetMathLibrary.MakeRotator` 0.0 0.0 (`KismetMathLibrary.SelectFloat` (`KismetMathLibrary.Lerp` 0.0 180.0 (`KismetMathLibrary.MapRangeClamped` (`self.GlobalTimeOfDay`) (`self.GetSunRiseTime`) (`self.GetSunSetTime`) 0.0 1.0)) (`KismetMathLibrary.Lerp` 180.0 360.0 (`KismetMathLibrary.SelectFloat` (`KismetMathLibrary.MapRangeClamped` (`self.GlobalTimeOfDay`) (`self.GetSunSetTime`) (+ (`self.GetSunRiseTime`) 24.0) 0.0 1.0) (`KismetMathLibrary.MapRangeClamped` (`self.GlobalTimeOfDay`) (- (`self.GetSunSetTime`) 24.0) (`self.GetSunRiseTime`) 0.0 1.0) (> (`self.GlobalTimeOfDay`) (`self.GetSunSetTime`)))) (not (or (> (`self.GlobalTimeOfDay`) (`self.GetSunSetTime`)) (< (`self.GlobalTimeOfDay`) (`self.GetSunRiseTime`)))))) false false)
  (`SceneComponent.K2_SetRelativeRotation` (`self.SkyAtmosphere`) (`KismetMathLibrary.MakeRotator` (* 0.0 0.75)) false false)
  (`SceneComponent.SetRelativeScale3D` (`self.Sun`) (`KismetMathLibrary.MakeVector` _returnvalue _returnvalue _returnvalue))
  (`LightComponent.SetIntensity` (`self.MoonLight`) (`KismetMathLibrary.MapRangeClamped` 0.0 0.0 1.0 1.0)))

(fn `UserConstructionScript`
  (bind _returnvalue (`PrimitiveComponent.CreateDynamicMaterialInstance` (`self.Sun`) 0 null "None"))
  (set `self.SunMaterial` _returnvalue)
  (bind _returnvalue_2 (`PrimitiveComponent.CreateDynamicMaterialInstance` (`self.Moon`) 0 null "None"))
  (set `self.MoonMaterial` _returnvalue_2)
  (`self.UpdateSky`)
  (`self.UpdateSky`))